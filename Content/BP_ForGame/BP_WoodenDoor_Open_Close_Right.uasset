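; Right-hand wooden door actor that the player swings with NumPad 2 while near it.
; Overlapping TriggerC enables input and prints a key hint; leaving disables input.
; The key plays the OpeningDoorRight timeline if its value times AngleDoor is non-negative, otherwise reverses it.
; Timeline updates set the WoodenDoorRight relative yaw to that product.
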(event OnComponentBeginOverlap(TriggerC)
  (params (OverlappedComponent :type Primitive%20Component%20Object%20Reference) (OtherActor :type Actor%20Object%20Reference) (OtherComp :type Primitive%20Component%20Object%20Reference) (OtherBodyIndex :type Integer) (bFromSweep :type Boolean) (SweepResult :type Hit%20Result%20Structure%20%28by%20ref%29))
  (Input|EnableInput (Game|GetPlayerController 0))
  (Development|PrintString "Press NumPad 2 to open right door"))

(event OnComponentEndOverlap(TriggerC)
  (params (OverlappedComponent :type Primitive%20Component%20Object%20Reference) (OtherActor :type Actor%20Object%20Reference) (OtherComp :type Primitive%20Component%20Object%20Reference) (OtherBodyIndex :type Integer))
  (Input|DisableInput (Game|GetPlayerController 0)))

(event Input|KeyboardEvents|NumPadTwo
  (params (Key :type Key%20Structure :default "None"))
  (:Pressed
    (if (>= (* (stale _opendoortime) (Variables|Default|GetAngleDoor)) 0.0)
      (bind _opendoortime (Timeline|OpeningDoorRight Play)
        (:Update
          (Transformation|SetRelativeRotation (Variables|Default|GetWoodenDoorRight) (Math|Rotator|MakeRotator 0.0 0.0 (* _opendoortime (Variables|Default|GetAngleDoor))) false false)))
      (else
        (Timeline|OpeningDoorRight Reverse)))))

(fn ConstructionScript)