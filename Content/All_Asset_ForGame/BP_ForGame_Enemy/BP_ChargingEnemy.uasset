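; BP_ChargingEnemy is an enemy that moves toward the side-scroller player character when it sees one.
; PawnSensing feeds sighted pawns through a cast to SideScrollerCharacter into AIMoveTo.
; On BeginPlay it detaches two position components, keeping world transforms, and sets an initial patrol target.
; SetPatrolPoint alternates the target between them via FlipFlop, but the Patrol event is empty, so nothing moves toward it.
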(event OnSeePawn(PawnSensing)
  (params (Pawn :type Pawn%20Object%20Reference))
  ;[1 1 1] Character Sense and Move
  (bind _asside_scroller_character (Utilities|Casting|CastToSideScrollerCharacter Pawn))
  (AI|AIMoveTo self "0, 0, 0" _asside_scroller_character 5.0 false))

(event Custom|SetPatrolPoint
  (Utilities|FlowControl|FlipFlop
    (:A
      (Variables|Default|SetTargetPatrolPoint (Transformation|GetWorldLocation (Variables|Default|GetPosition1))))
    (:B
      (Variables|Default|SetTargetPatrolPoint (Transformation|GetWorldLocation (Variables|Default|GetPosition2))))))

(event Custom|Patrol)

(event EventBeginPlay
  ;[1 1 1] Create Patrol Points
  (Transformation|DetachFromComponent (Variables|Default|GetPosition1) "KeepWorld" "KeepWorld" "KeepWorld" true)
  (CallFunction|SetPatrolPoint))

(fn ConstructionScript)