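; BP_WoodenDoor_Open_Close is a wooden door, described as the left door, that the player opens and closes with R.
; Overlapping TriggerDoor enables input for player 0 and prints an on-screen key hint, and leaving it disables input.
; R plays or reverses the OpeningDoor timeline based on whether its value times Angle is at or below zero.
; That same product drives the door's relative yaw.
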(event OnComponentBeginOverlap(TriggerDoor)
  (params (OverlappedComponent :type Primitive%20Component%20Object%20Reference) (OtherActor :type Actor%20Object%20Reference) (OtherComp :type Primitive%20Component%20Object%20Reference) (OtherBodyIndex :type Integer) (bFromSweep :type Boolean) (SweepResult :type Hit%20Result%20Structure%20%28by%20ref%29))
  ;[1 1 1] Open/Close left door
  (Input|EnableInput (Game|GetPlayerController 0))
  (Development|PrintString "Press \"R\" Key to open left door"))

(event OnComponentEndOverlap(TriggerDoor)
  (params (OverlappedComponent :type Primitive%20Component%20Object%20Reference) (OtherActor :type Actor%20Object%20Reference) (OtherComp :type Primitive%20Component%20Object%20Reference) (OtherBodyIndex :type Integer))
  ;[1 1 1] Open/Close left door
  (Input|DisableInput (Game|GetPlayerController 0)))

(event EventBeginPlay)

(event Collision|EventActorBeginOverlap
  (params (OtherActor :type Actor%20Object%20Reference)))

(event EventTick
  (params (DeltaSeconds :type Float%20%28single-precision%29)))

(event Input|KeyboardEvents|R
  (params (Key :type Key%20Structure :default "None"))
  ;[1 1 1] Open/Close left door
  (:Pressed
    (if (<= (* (stale _opendoortime) (Variables|Default|GetAngle)) 0.0)
      (bind _opendoortime (Timeline|OpeningDoor Play)
        (:Update
          (Transformation|SetRelativeRotation (Variables|Default|GetWoodenDoor) (Math|Rotator|MakeRotator 0.0 0.0 (* _opendoortime (Variables|Default|GetAngle))) false false)))
      (else
        (Timeline|OpeningDoor Reverse)))))

(fn ConstructionScript)