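; BP_MovingFloor is a moving floor platform that starts moving on BeginPlay.
; The MoveFloor timeline's track, scaled by LeftToRight, sets the MovingFloor component's relative location on each update.
; ForXYorZ selects X, Y or Z, with other values above one falling through to a combined Y and Z move.
; When the timeline finishes, comparing the scaled value to LeftToRight chooses between Reverse and Play.
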(event EventBeginPlay
  (bind _movingfloor (Variables|Default|GetMovingFloor))
  (bind _forxyorz (Variables|Default|GetForXYorZ))
  (bind _lefttoright (Variables|Default|GetLeftToRight))
  ;[1 1 1] Moving Floor
  ;;[1 1 1] Distance the floor is moving
  (bind _movingfloortile (Timeline|MoveFloor Play)
    (:Update
      ;;[1 1 1] Determine Which dir. floor is moving
      (if (<= _forxyorz 1.0)
        (Transformation|SetRelativeLocation _movingfloor (Math|Vector|MakeVector (* _movingfloortile _lefttoright) 0.0 0.0) false false)
        (elif (== _forxyorz 2.0)
          (Transformation|SetRelativeLocation _movingfloor (Math|Vector|MakeVector 0.0 (* _movingfloortile _lefttoright) 0.0) false false)
          (elif (== _forxyorz 3.0)
            (Transformation|SetRelativeLocation _movingfloor (Math|Vector|MakeVector 0.0 0.0 (* _movingfloortile _lefttoright)) false false)
            (else
              (if (== _forxyorz 4.0)
                _
                (else
                  _))
              (Transformation|SetRelativeLocation _movingfloor (Math|Vector|MakeVector 0.0 (* _movingfloortile _lefttoright) (* _movingfloortile _lefttoright)) false false))))))
    (:Finished
      (if (<= (* _movingfloortile _lefttoright) _lefttoright)
        (Timeline|MoveFloor Reverse)
        (else
          (Timeline|MoveFloor Play))))))

(fn ConstructionScript)