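; Music manager Blueprint that plays a list of tracks and switches which one is audible.
; On BeginPlay it creates a 2D sound for every TrackList entry and starts them all at once at zero volume, then raises the chosen starting track to the music volume.
; The changemusicto event mutes the current track and unmutes the requested index, an instant switch without fades that leaves every track running.
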(event Custom|change%20music%20to
  (params (Index%20song%20of%20play :type Integer))
  (bind _musicreference_ (Variables|Default|Getmusicreference%20))
  (bind _output (Utilities|Array|Get(acopy) _musicreference_ Index%20song%20of%20play))
  (Audio|Components|Audio|SetVolumeMultiplier (Variables|Default|Getcurrent%20music%20ref) 0.0 :!class /Script/Engine.AudioComponent)
  (Audio|Components|Audio|SetVolumeMultiplier _output (Variables|Default|Getmusicvolumen) :!class /Script/Engine.AudioComponent)
  (Variables|Default|Setcurrent%20music%20ref _output))

(event EventBeginPlay
  (bind _indexsong_to_play_on_levelbegin (Variables|Default|GetIndexsong%20to%20play%20on%20levelbegin))
  (bind _musicreference_ (Variables|Default|Getmusicreference%20))
  (bind _output (Utilities|Array|Get(acopy) _musicreference_ _indexsong_to_play_on_levelbegin))
  (for _array_element (Variables|Default|GetTrackList)
    (bind _returnvalue (Audio|CreateSound2D _array_element 1.0 1.0 0.0 0))
    (Utilities|Array|Add (Variables|Default|Getmusicreference%20) _returnvalue)
    (Audio|Components|Audio|SetVolumeMultiplier _returnvalue 0.0 :!class /Script/Engine.AudioComponent)
    (Audio|Components|Audio|Play _returnvalue 0.0))
  (Audio|Components|Audio|SetVolumeMultiplier _output (Variables|Default|Getmusicvolumen) :!class /Script/Engine.AudioComponent)
  (Variables|Default|Setcurrent%20music%20ref _output))

(fn ConstructionScript)