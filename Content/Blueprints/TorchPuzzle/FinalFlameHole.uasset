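; FinalFlameHole is the torch puzzle's final socket, which opens a large double door when the FinalFlamePeg is placed in it.
; On BeginPlay it clears its Occupied flag, deactivates its fire particle and zeroes its point light.
; When its Box overlaps a FinalFlamePeg, it sets Occupied, lights the fire and light, and snaps both door meshes to new rotations without animation.
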(event OnComponentBeginOverlap(Box)
  (params (OverlappedComponent :type Primitive%20Component%20Object%20Reference) (OtherActor :type Actor%20Object%20Reference) (OtherComp :type Primitive%20Component%20Object%20Reference) (OtherBodyIndex :type Integer) (bFromSweep :type Boolean) (SweepResult :type Hit%20Result%20Structure%20%28by%20ref%29))
  (if (== (Utilities|GetClass OtherActor) "/Game/Blueprints/TorchPuzzle/FinalFlamePeg.FinalFlamePeg_C")
    (Variables|Default|SetOccupied true)
    (bind _output_get (Variables|Default|SetP_Fire (Variables|Default|GetP_Fire)))
    (Components|Activation|SetActive _output_get true false)
    (bind _output_get_2 (Variables|Default|SetPointLight (Variables|Default|GetPointLight)))
    (Rendering|Components|Light|SetIntensity _output_get_2 1e+04)
    (Transformation|SetRelativeRotation (Variables|Default|GetSM_DoorWay_Large_Door_Left) (Math|Rotator|MakeRotator 0.0 0.0 0.0) false false)
    (Transformation|SetRelativeRotation (Variables|Default|GetSM_DoorWay_Large_Door_Right) (Math|Rotator|MakeRotator 0.0 0.0 1.8e+02) false false)))

(event EventBeginPlay
  (Variables|Default|SetOccupied false)
  (bind _output_get (Variables|Default|SetP_Fire (Variables|Default|GetP_Fire)))
  (Components|Activation|SetActive _output_get false false)
  (bind _output_get_2 (Variables|Default|SetPointLight (Variables|Default|GetPointLight)))
  (Rendering|Components|Light|SetIntensity _output_get_2 0.0))

(event Collision|EventActorBeginOverlap
  (params (OtherActor :type Actor%20Object%20Reference)))

(event EventTick
  (params (DeltaSeconds :type Float%20%28single-precision%29)))

(fn ConstructionScript)