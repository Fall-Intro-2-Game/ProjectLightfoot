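; Left half of a puzzle door that swings open when its matching puzzle is solved and closed when it is not.
; It finds its BP_PuzzleDoor_Counter by searching all counters for the same PuzzleNumber.
; DoorStatusChanged, called from that counter, reads Solved and plays or reverses a timeline that yaws WoodenDoor by Angle.
; On puzzle doors, player overlap with TriggerDoor prints how many torches must be lit, using the counter's PuzzleHoles.
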(event OnComponentBeginOverlap(TriggerDoor)
  (params (OverlappedComponent :type Primitive%20Component%20Object%20Reference) (OtherActor :type Actor%20Object%20Reference) (OtherComp :type Primitive%20Component%20Object%20Reference) (OtherBodyIndex :type Integer) (bFromSweep :type Boolean) (SweepResult :type Hit%20Result%20Structure%20%28by%20ref%29))
  ;[1 1 1] If Player Enters Doorspace, print string number of puzzle slots there are for this door
  (if (Variables|Default|GetIsPuzzle)
    (if (== (Utilities|GetClass OtherActor) "/Game/SideScrollerBP/Blueprints/SideScrollerCharacter.SideScrollerCharacter_C")
      (bind _outactors (Actor|GetAllActorsOfClass "/Game/Blueprints/Puzzles/BP_PuzzleDoor_Counter.BP_PuzzleDoor_Counter_C"))
      (bind (_array_element _array_index) (Utilities|Array|ForEachLoopwithBreak _outactors :!label _label)
        (:LoopBody
          (if (== (Variables|/Game/Blueprints/Puzzles/BP_PuzzleDoor_Counter.BP_PuzzleDoor_Counter_C|GetPuzzleNumber _array_element) (Variables|Default|GetPuzzleNumber))
            (goto _label Break)))
        (:Completed
          (Development|PrintString (Utilities|String|Append (Utilities|String|Append "Light " (Utilities|String|ToString(Integer) (Variables|/Game/Blueprints/Puzzles/BP_PuzzleDoor_Counter.BP_PuzzleDoor_Counter_C|GetPuzzleHoles (Utilities|Array|Get(acopy) _outactors _array_index)))) " torches to open this door.")))))))

(event OnComponentEndOverlap(TriggerDoor)
  (params (OverlappedComponent :type Primitive%20Component%20Object%20Reference) (OtherActor :type Actor%20Object%20Reference) (OtherComp :type Primitive%20Component%20Object%20Reference) (OtherBodyIndex :type Integer))
  ;[1 1 1] If Player Enters Doorspace, print string number of puzzle slots there are for this door
)

(event Custom|DoorStatusChanged
  ;[1 1 1] Door Status Changed - Open/Close left door - Called from BP_PuzzleDoor_Counter
  (bind _outactors (Actor|GetAllActorsOfClass "/Game/Blueprints/Puzzles/BP_PuzzleDoor_Counter.BP_PuzzleDoor_Counter_C"))
  (bind _array_element (Utilities|Array|ForEachLoopwithBreak _outactors)
    (:LoopBody
      (if (== (Variables|/Game/Blueprints/Puzzles/BP_PuzzleDoor_Counter.BP_PuzzleDoor_Counter_C|GetPuzzleNumber _array_element) (Variables|Default|GetPuzzleNumber))
        (if (Variables|/Game/Blueprints/Puzzles/BP_PuzzleDoor_Counter.BP_PuzzleDoor_Counter_C|GetSolved _array_element)
          (bind _opendoortime (Timeline|Timeline_0 Play)
            (:Update
              (Transformation|SetRelativeRotation (Variables|Default|GetWoodenDoor) (Math|Rotator|MakeRotator 0.0 0.0 (* _opendoortime (Variables|Default|GetAngle))) false false)))
          (else
            (Timeline|Timeline_0 Reverse)))))))

(event EventBeginPlay)

(event Collision|EventActorBeginOverlap
  (params (OtherActor :type Actor%20Object%20Reference)))

(event EventTick
  (params (DeltaSeconds :type Float%20%28single-precision%29)))

(event Input|KeyboardEvents|NumPadOne
  (params (Key :type Key%20Structure))
  ;[1 1 1] Code from original Door BP - Disabled
)

(fn ConstructionScript)