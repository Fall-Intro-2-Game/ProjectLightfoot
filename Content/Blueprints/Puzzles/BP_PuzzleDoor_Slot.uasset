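; BP_PuzzleDoor_Slot is a door-puzzle socket that lights its torch while a peg with the same PuzzleNumber sits in it.
; BeginPlay turns the torch off and finds the BP_PuzzleDoor_Counter sharing that number.
; Box overlap begin and end events toggle Occupied for matching BP_PuzzleDoor_Pegs, switch the particles and point light, and notify that counter through PuzzleCountChanged.
; Unconnected PrintString debug copies of the overlap logic never run.
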(event OnComponentBeginOverlap(BoxCollider)
  (params (OverlappedComponent :type Primitive%20Component%20Object%20Reference) (OtherActor :type Actor%20Object%20Reference) (OtherComp :type Primitive%20Component%20Object%20Reference) (OtherBodyIndex :type Integer) (bFromSweep :type Boolean) (SweepResult :type Hit%20Result%20Structure%20%28by%20ref%29))
  ;[1 1 1] Something Entered the Puzzle Space - See if it is BP_PuzzleDoor_Peg - Update Status
  (if (not (Variables|Default|GetOccupied))
    (if (== (Utilities|GetClass OtherActor) "/Game/Blueprints/Puzzles/BP_PuzzleDoor_Peg.BP_PuzzleDoor_Peg_C")
      (if (== (Variables|Default|GetPuzzleNumber) (Variables|/Game/Blueprints/Puzzles/BP_PuzzleDoor_Peg.BP_PuzzleDoor_Peg_C|GetPuzzleNumber (.AsBP%20Puzzle%20Door%20Peg (Utilities|Casting|CastToBP_PuzzleDoor_Peg OtherActor))))
        (Variables|Default|SetOccupied true)
        (Default|PuzzleCountChanged (Variables|Default|GetPuzzleSolved))
        (bind _output_get (Variables|Default|SetParticleSystem (Variables|Default|GetParticleSystem)))
        (Components|Activation|SetActive _output_get true false)
        (bind _output_get_2 (Variables|Default|SetPointLight (Variables|Default|GetPointLight)))
        (Rendering|Components|Light|SetIntensity _output_get_2 5e+03)))))

(event OnComponentEndOverlap(BoxCollider)
  (params (OverlappedComponent :type Primitive%20Component%20Object%20Reference) (OtherActor :type Actor%20Object%20Reference) (OtherComp :type Primitive%20Component%20Object%20Reference) (OtherBodyIndex :type Integer))
  ;[1 1 1] Something Left the Puzzle Space - See if it is BP_PuzzleDoor_Peg - Update Status
  (if (Variables|Default|GetOccupied)
    (if (== (Utilities|GetClass OtherActor) "/Game/Blueprints/Puzzles/BP_PuzzleDoor_Peg.BP_PuzzleDoor_Peg_C")
      (if (== (Variables|Default|GetPuzzleNumber) (Variables|/Game/Blueprints/Puzzles/BP_PuzzleDoor_Peg.BP_PuzzleDoor_Peg_C|GetPuzzleNumber (.AsBP%20Puzzle%20Door%20Peg (Utilities|Casting|CastToBP_PuzzleDoor_Peg OtherActor))))
        (Variables|Default|SetOccupied false)
        (Default|PuzzleCountChanged (Variables|Default|GetPuzzleSolved))
        (bind _output_get (Variables|Default|SetParticleSystem (Variables|Default|GetParticleSystem)))
        (Components|Activation|SetActive _output_get false false)
        (bind _output_get_2 (Variables|Default|SetPointLight (Variables|Default|GetPointLight)))
        (Rendering|Components|Light|SetIntensity _output_get_2 0.0)))))

(event EventBeginPlay
  ;[1 1 1] Start Game / Turn Off My Torch / Find My Puzzle Group Leader
  (bind _output_get (Variables|Default|SetParticleSystem (Variables|Default|GetParticleSystem)))
  (Components|Activation|SetActive _output_get false false)
  (bind _output_get_2 (Variables|Default|SetPointLight (Variables|Default|GetPointLight)))
  (Rendering|Components|Light|SetIntensity _output_get_2 0.0)
  (Variables|Default|SetOccupied false)
  (bind _outactors (Actor|GetAllActorsOfClass "/Game/Blueprints/Puzzles/BP_PuzzleDoor_Counter.BP_PuzzleDoor_Counter_C"))
  (bind _array_element (Utilities|Array|ForEachLoopwithBreak _outactors)
    (:LoopBody
      (if (== (Variables|/Game/Blueprints/Puzzles/BP_PuzzleDoor_Counter.BP_PuzzleDoor_Counter_C|GetPuzzleNumber _array_element) (Variables|Default|GetPuzzleNumber))
        (Variables|Default|SetPuzzleSolved _array_element)))))

(event Collision|EventActorBeginOverlap
  (params (OtherActor :type Actor%20Object%20Reference)))

(event EventTick
  (params (DeltaSeconds :type Float%20%28single-precision%29)))

(fn ConstructionScript)