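; Per-puzzle counter actor that tracks whether every slot sharing its PuzzleNumber is filled and notifies that puzzle's doors.
; On BeginPlay it caches all left doors, right doors and slots in the level, then counts the slots matching its number.
; Slots call PuzzleCountChanged, which recounts occupied slots and updates Solved.
; Matching doors get DoorStatusChanged whenever the puzzle evaluates as solved or becomes unsolved.
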(event Custom|PuzzleCountChanged
  (bind _puzzlenumber (Variables|Default|GetPuzzleNumber))
  ;[1 1 1] Status Changed - Called from BP_PuzzleDoor_Slot
  ;;[1 1 1] See if all the slots are filled
  (Variables|Default|SetCorrectlyFilled 0)
  (for _array_element (Variables|Default|GetSquareHoles)
    (if (== (Variables|/Game/Blueprints/Puzzles/BP_PuzzleDoor_Slot.BP_PuzzleDoor_Slot_C|GetPuzzleNumber _array_element) (Variables|Default|GetPuzzleNumber))
      (if (Variables|/Game/Blueprints/Puzzles/BP_PuzzleDoor_Slot.BP_PuzzleDoor_Slot_C|GetOccupied _array_element)
        (Math|Integer|IncrementInt (Variables|Default|GetCorrectlyFilled)))))
  (if (== (Variables|Default|GetPuzzleHoles) (Variables|Default|GetCorrectlyFilled))
    (Variables|Default|SetSolved true)
    ;;[1 1 1] Tell The Doors to Check
    (for _array_element_2 (Variables|Default|GetPuzzleDoorsLeft) :!label _label
      (if (== (Variables|/Game/Blueprints/Puzzles/BP_PuzzleDoor_Left.BP_PuzzleDoor_Left_C|GetPuzzleNumber _array_element_2) _puzzlenumber)
        (Default|DoorStatusChanged _array_element_2)))
    (for _array_element_3 (Variables|Default|GetPuzzleDoorsRight)
      (if (== _puzzlenumber (Variables|/Game/Blueprints/Puzzles/BP_PuzzleDoor_Right.BP_PuzzleDoor_Right_C|GetPuzzleNumber _array_element_3))
        (Default|DoorStatusChanged _array_element_3)))
    (elif (Variables|Default|GetSolved)
      (Variables|Default|SetSolved false)
      (goto _label))))

(event EventBeginPlay
  ;[1 1 1] Get References to All Puzzle Doors
  (bind _outactors (Actor|GetAllActorsOfClass "/Game/Blueprints/Puzzles/BP_PuzzleDoor_Left.BP_PuzzleDoor_Left_C"))
  (Variables|Default|SetPuzzleDoorsLeft _outactors)
  (bind _outactors_2 (Actor|GetAllActorsOfClass "/Game/Blueprints/Puzzles/BP_PuzzleDoor_Right.BP_PuzzleDoor_Right_C"))
  (Variables|Default|SetPuzzleDoorsRight _outactors_2)
  ;[1 1 1] Count Puzzle Objects and Set Initial Values for Each Puzzle
  (Variables|Default|SetPuzzleHoles 0)
  (Variables|Default|SetCorrectlyFilled 0)
  (bind _outactors_3 (Actor|GetAllActorsOfClass "/Game/Blueprints/Puzzles/BP_PuzzleDoor_Slot.BP_PuzzleDoor_Slot_C"))
  (bind _output_get (Variables|Default|SetSquareHoles _outactors_3))
  (for _array_element _output_get
    (if (== (Variables|/Game/Blueprints/Puzzles/BP_PuzzleDoor_Slot.BP_PuzzleDoor_Slot_C|GetPuzzleNumber _array_element) (Variables|Default|GetPuzzleNumber))
      (bind _result (Math|Integer|IncrementInt (Variables|Default|GetPuzzleHoles))
        (:%20%20
          (Variables|Default|SetPuzzleHoles _result))))))

(event Collision|EventActorBeginOverlap
  (params (OtherActor :type Actor%20Object%20Reference)))

(event EventTick
  (params (DeltaSeconds :type Float%20%28single-precision%29)))

(fn ConstructionScript)