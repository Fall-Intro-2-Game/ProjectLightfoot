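; BP_PuzzleDoor_Right is the right half of a puzzle-locked wooden door that swings open when its puzzle is solved.
; DoorStatusChanged, called by BP_PuzzleDoor_Counter, finds the counter with the matching PuzzleNumber and plays or reverses a rotation timeline based on its Solved state.
; On puzzle doors, a SideScrollerCharacter entering TriggerC sees a printed count of torches to light.
; An older NumPad 2 toggle remains, with its input enabling disconnected.
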(event OnComponentBeginOverlap(TriggerC)
  (params (OverlappedComponent :type Primitive%20Component%20Object%20Reference) (OtherActor :type Actor%20Object%20Reference) (OtherComp :type Primitive%20Component%20Object%20Reference) (OtherBodyIndex :type Integer) (bFromSweep :type Boolean) (SweepResult :type Hit%20Result%20Structure%20%28by%20ref%29))
  ;[1 1 1] If Player Enters Doorspace, print string number of puzzle slots there are for this door
  (if (Variables|Default|GetIsPuzzle)
    (if (== (Utilities|GetClass OtherActor) "/Game/SideScrollerBP/Blueprints/SideScrollerCharacter.SideScrollerCharacter_C")
      (bind _outactors (Actor|GetAllActorsOfClass "/Game/Blueprints/Puzzles/BP_PuzzleDoor_Counter.BP_PuzzleDoor_Counter_C"))
      (bind (_array_element _array_index) (Utilities|Array|ForEachLoopwithBreak _outactors :!label _label)
        (:LoopBody
          (if (== (Variables|/Game/Blueprints/Puzzles/BP_PuzzleDoor_Counter.BP_PuzzleDoor_Counter_C|GetPuzzleNumber _array_element) (Variables|Default|GetPuzzleNumber))
            (goto _label Break)))
        (:Completed
          (Development|PrintString (Utilities|String|Append (Utilities|String|Append "Light " (Utilities|String|ToString(Integer) (Variables|/Game/Blueprints/Puzzles/BP_PuzzleDoor_Counter.BP_PuzzleDoor_Counter_C|GetPuzzleHoles (Utilities|Array|Get(acopy) _outactors _array_index)))) " torches to open the door.")))))))

(event OnComponentEndOverlap(TriggerC)
  (params (OverlappedComponent :type Primitive%20Component%20Object%20Reference) (OtherActor :type Actor%20Object%20Reference) (OtherComp :type Primitive%20Component%20Object%20Reference) (OtherBodyIndex :type Integer))
  ;[1 1 1] Original Door Logic- Disabled
)

(event Custom|DoorStatusChanged
  ;[1 1 1] Door Status Changed - Open/Close right door - Called from BP_PuzzleDoor_Counter
  (bind _outactors (Actor|GetAllActorsOfClass "/Game/Blueprints/Puzzles/BP_PuzzleDoor_Counter.BP_PuzzleDoor_Counter_C"))
  (bind _array_element (Utilities|Array|ForEachLoopwithBreak _outactors)
    (:LoopBody
      (if (== (Variables|/Game/Blueprints/Puzzles/BP_PuzzleDoor_Counter.BP_PuzzleDoor_Counter_C|GetPuzzleNumber _array_element) (Variables|Default|GetPuzzleNumber))
        (if (Variables|/Game/Blueprints/Puzzles/BP_PuzzleDoor_Counter.BP_PuzzleDoor_Counter_C|GetSolved _array_element)
          (bind _opendoortime (Timeline|Timeline_0 Play)
            (:Update
              (Transformation|SetRelativeRotation (Variables|Default|GetWoodenDoorRight) (Math|Rotator|MakeRotator 0.0 0.0 (* _opendoortime (Variables|Default|GetAngleDoor))) false false)))
          (else
            (Timeline|Timeline_0 Reverse)))))))

(event EventBeginPlay)

(event Input|KeyboardEvents|NumPadTwo
  (params (Key :type Key%20Structure))
  ;[1 1 1] Original Door Logic- Disabled
  (:Pressed
    (if (>= (* (stale _opendoortime) (Variables|Default|GetAngleDoor)) 0.0)
      (bind _opendoortime (Timeline|OpeningDoorRight Play)
        (:Update
          (Transformation|SetRelativeRotation (Variables|Default|GetWoodenDoorRight) (Math|Rotator|MakeRotator 0.0 0.0 (* _opendoortime (Variables|Default|GetAngleDoor))) false false)))
      (else
        (Timeline|OpeningDoorRight Reverse)))))

(fn ConstructionScript)